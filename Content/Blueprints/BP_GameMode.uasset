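; Game mode that sets up the player's UI and owns the item inventory.
; On BeginPlay it creates the menu and HUD widgets and hands them, with itself, to the player's BP_Character.
; AddItem stacks quantities onto entries with a matching name or appends a new one, then refreshes that slot in the menu widget.
; A debug event prints the inventory.
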(event Custom|AddItem
  (params (ItemInfo :type DA%20Item%20Object%20Reference) (Number :type Integer))
  (bind _index (CallFunction|AddItemtoArray ItemInfo Number))
  (Default|UpdateInventory (Variables|Default|GetMenuWidget) (Utilities|Array|Get(acopy) (Variables|Default|GetInventory) _index) _index))

(event Custom|showinventory
  ;[1 1 1] Debug
  (for _array_element (Variables|Default|GetInventory)
    (Development|PrintString (Utilities|String|Append (Utilities|String|ToString(Text) (.Name (Utilities|Struct|BreakInventoryEntry _array_element))) (Utilities|String|ToString(Integer) (.Number (Utilities|Struct|BreakInventoryEntry _array_element)))))))

(event EventBeginPlay
  (bind _returnvalue (Game|ConstructObjectfromClass "/Game/Widgets/WBP_UI.WBP_UI_C"))
  (bind _output_get (Variables|Default|SetMenuWidget _returnvalue))
  (UserInterface|Viewport|AddtoViewport _output_get 5)
  (bind _asbp_character (Utilities|Casting|CastToBP_Character (Game|Player|GetPlayerPawn 0))
    (:then
      (Variables|Default|SetBP_Character _asbp_character))
    (:CastFailed
      (Development|PrintString "Error : CastFailed to BP_Chara")))
  (bind _returnvalue_2 (Game|ConstructObjectfromClass "/Game/Widgets/WBP_HUD.WBP_HUD_C"))
  (bind _output_get_2 (Variables|Default|SetHUDWidget _returnvalue_2))
  (UserInterface|Viewport|AddtoViewport _output_get_2 2)
  (Default|SetbyGameMode (Variables|Default|GetBP_Character) (Variables|Default|GetMenuWidget) (Variables|Default|GetHUDWidget) self))

(fn ConstructionScript)

(fn AddItemtoArray
  (params (ItemInfo :type DA%20Item%20Object%20Reference) (Number :type Integer))
  (bind _inventory (Variables|Default|GetInventory))
  (for (_array_element _array_index) _inventory
    (if (Utilities|Enum|Equal(Enum) (.Name (Utilities|Struct|BreakInventoryEntry _array_element)) (Variables|/Game/Blueprints/DA_Item.DA_Item_C|GetName ItemInfo))
      (|SetBy-RefVar (Utilities|Array|Get(acopy) (Variables|Default|GetInventory) _array_index) (Utilities|Struct|MakeInventoryEntry (.Name (Utilities|Struct|BreakInventoryEntry _array_element)) (.Type (Utilities|Struct|BreakInventoryEntry _array_element)) (.Rarity (Utilities|Struct|BreakInventoryEntry _array_element)) (+ Number (.Number (Utilities|Struct|BreakInventoryEntry _array_element)))))
      (return _array_index)))
  (bind _returnvalue (Utilities|Array|Add _inventory (Utilities|Struct|MakeInventoryEntry (Variables|/Game/Blueprints/DA_Item.DA_Item_C|GetName ItemInfo) (Variables|/Game/Blueprints/DA_Item.DA_Item_C|GetType ItemInfo) (Variables|/Game/Blueprints/DA_Item.DA_Item_C|GetRarity ItemInfo) Number)))
  (return _returnvalue))