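; BP_Item is an item actor that highlights itself when the player character comes within range.
; It caches the player's BP_Character on BeginPlay and uses a Sphere overlap to toggle the outline when that character enters or leaves.
; Outlining sets or clears the MM_ItemOutline overlay material on the Cube, and each change calls AddOutlinedItem or RemoveOutlinedItem on the character.
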(event OnComponentBeginOverlap(Sphere)
  (params (OverlappedComponent :type Primitive%20Component%20Object%20Reference) (OtherActor :type Actor%20Object%20Reference) (OtherComp :type Primitive%20Component%20Object%20Reference) (OtherBodyIndex :type Integer) (bFromSweep :type Boolean) (SweepResult :type Hit%20Result%20Structure%20%28by%20ref%29))
  (if (== OtherActor (Game|GetPlayerCharacter 0))
    (CallFunction|Outline true)
    (Default|AddOutlinedItem (Variables|Default|GetBP%20Character))))

(event OnComponentEndOverlap(Sphere)
  (params (OverlappedComponent :type Primitive%20Component%20Object%20Reference) (OtherActor :type Actor%20Object%20Reference) (OtherComp :type Primitive%20Component%20Object%20Reference) (OtherBodyIndex :type Integer))
  (if (== (Game|GetPlayerCharacter 0) OtherActor)
    (CallFunction|Outline false)
    (Default|RemoveOutlinedItem (Variables|Default|GetBP%20Character))))

(event EventBeginPlay
  (bind _asbp_character (Utilities|Casting|CastToBP_Character (Game|GetPlayerCharacter 0)))
  (Variables|Default|SetBP%20Character _asbp_character))

(fn ConstructionScript)

(fn Outline
  (params (Outline :type Boolean))
  (bind _cube (Variables|Default|GetCube))
  (bind _output_get (Variables|Default|SetIsOutlined Outline))
  (if _output_get
    (Rendering|Material|SetOverlayMaterial _cube "/Game/Assets/Material/MM_ItemOutline.MM_ItemOutline" :!class /Script/Engine.MeshComponent)
    (else
      (Rendering|Material|SetOverlayMaterial _cube 0 :!class /Script/Engine.MeshComponent))))